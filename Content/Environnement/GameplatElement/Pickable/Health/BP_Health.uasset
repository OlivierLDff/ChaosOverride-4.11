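; BP_Health is a health pickup that heals a COCharacter entering its sphere, then respawns in place.
; The sphere overlap runs on the server only, checks the Active flag and calls the character's HealBlueprint with the Health amount and no refill.
; When the heal succeeds, it hides the mesh and deactivates for a fixed delay, then becomes visible and active again.
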(event `self.ReceiveBeginPlay`)

(event `self.ReceiveActorBeginOverlap`
  (params (OtherActor :type "Actor Object Reference")))

(event `self.ReceiveTick`
  (params (DeltaSeconds :type "Float (single-precision)")))

(event `self.Sphere.OnComponentBeginOverlap`
  (params (OtherActor :type "Actor Object Reference") (OtherComp :type "PrimitiveComponent Object Reference") (OtherBodyIndex :type Integer) (bFromSweep :type Boolean) (SweepResult :type "HitResult Structure (by ref)"))
  (`/Engine/EditorBlueprintResources/ActorMacros.Switch Has Authority`
    (:`Authority`
      (if (`self.bActive`)
        (if (!= OtherActor self)
          (bind _ascocharacter (cast `COCharacter` OtherActor))
          (bind _returnvalue (`COCharacter.HealBlueprint` _ascocharacter (`KismetMathLibrary.Conv_IntToDouble` (`self.Health`)) false))
          (if _returnvalue
            (`SceneComponent.SetVisibility` (`self.StaticMesh`) false false)
            (set `self.bActive` false)
            (`KismetSystemLibrary.Delay` 5.0)
            (set `self.bActive` true)
            (`SceneComponent.SetVisibility` (`self.StaticMesh`) true false)))))))

(fn `UserConstructionScript`)