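; BP_AmmoBox is an ammo pickup that refills a character's weapon ammo, then reappears after a short delay.
; On sphere overlap, the authority asks the COCharacter's Inventory to refill the configured weapon class with the set ammo amount.
; A successful refill hides the root and its children and clears the Active flag until the delay restores both, so the box is reused rather than destroyed.
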(event `self.ReceiveBeginPlay`)

(event `self.ReceiveActorBeginOverlap`
  (params (OtherActor :type "Actor Object Reference")))

(event `self.ReceiveTick`
  (params (DeltaSeconds :type "Float (single-precision)")))

(event `self.Sphere.OnComponentBeginOverlap`
  (params (OtherActor :type "Actor Object Reference") (OtherComp :type "PrimitiveComponent Object Reference") (OtherBodyIndex :type Integer) (bFromSweep :type Boolean) (SweepResult :type "HitResult Structure (by ref)"))
  (`/Engine/EditorBlueprintResources/ActorMacros.Switch Has Authority`
    (:`Authority`
      (if (`self.active`)
        (if (!= OtherActor self)
          (bind _ascocharacter (cast `COCharacter` OtherActor))
          (bind _returnvalue (`COInventoryComponent.RefillAmmoBlueprint` (`COCharacter.Inventory` _ascocharacter) (`self.WeaponClass`) (`self.ammo`)))
          (if _returnvalue
            (`SceneComponent.SetVisibility` (`self.DefaultSceneRoot`) false true)
            (set `self.active` false)
            (`KismetSystemLibrary.Delay` 5.0)
            (`SceneComponent.SetVisibility` (`self.DefaultSceneRoot`) true true)
            (set `self.active` true)))))))

(fn `UserConstructionScript`)