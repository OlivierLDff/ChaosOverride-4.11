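; BP_COPlayerController is a player controller that handles score display, the pause menu and a spectator switch.
; Holding Select shows an IGScore widget on the player's screen until release, while Start adds a new IG_PauseMenu widget to the viewport.
; The hardcoded A key prints the controlled pawn's name, then spawns and possesses a SpectatorPawn snapped to a random COCharacter's capsule, apparently for debugging.
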(event `self.ReceiveBeginPlay`)

(event `self.ReceiveTick`
  (params (DeltaSeconds :type "Float (single-precision)")))

(event `InputAction|Select`
  (params (Key :type "Key Structure" :default "AnyKey"))
  (:`Pressed`
    (bind _returnvalue (`|CreateWidget` "/Game/HUD/IGHUD/IGScore/IGScore.IGScore_C" self))
    (`UserWidget.AddToPlayerScreen` _returnvalue 0))
  (:`Released`
    (`Widget.RemoveFromParent` _returnvalue)))

(event `InputAction|Start`
  (params (Key :type "Key Structure" :default "AnyKey"))
  ;[1 1 1] Start
  (:`Pressed`
    (bind _returnvalue (`|CreateWidget` "/Game/HUD/IGHUD/IG_PauseMenu.IG_PauseMenu_C" self))
    (`UserWidget.AddToViewport` _returnvalue 0)))

(event `Key|A`
  (params (Key :type "Key Structure" :default "AnyKey"))
  (:`Pressed`
    (`KismetSystemLibrary.PrintString` (`KismetSystemLibrary.GetObjectName` (`self.K2_GetPawn`)))
    (bind _returnvalue (`|SpawnActorFromClass` "/Script/Engine.SpectatorPawn" (`KismetMathLibrary.MakeTransform` (0.0 0.0 200.0) (struct)) "Undefined" "OverrideRootScale"))
    (`self.Possess` _returnvalue)
    (bind _outactors (`GameplayStatics.GetAllActorsOfClass` "/Script/ChaosOverride.COCharacter"))
    (`self.K2_AttachRootComponentTo` _returnvalue (`Character.CapsuleComponent` (`KismetArrayLibrary.Array_Get` _outactors (`KismetMathLibrary.RandomIntegerInRange` 0 (- (`KismetArrayLibrary.Array_Length` _outactors) 1)))) "None" "SnapToTargetIncludingScale" true)))

(fn `UserConstructionScript`)