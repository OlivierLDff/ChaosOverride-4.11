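; AI controller that runs a behavior tree on possess and picks its pawn's target from AI Perception.
; On perception updates or target death, it keeps a living, visible current target, otherwise takes the first living actor seen, then the nearest recently heard.
; Results go to Blackboard keys for target, sight flag and search time.
; Heard or lost living targets get a search time, while dead targets are cleared.
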(event OnPerceptionUpdated(AIPerception)
  (params (UpdatedActors :type Array%20of%20Actor%20Object%20References))
  ;[1 1 1] The new target is the current target or the last sound heard
  (bind _output_get (Variables|Default|SetPerceptedActors UpdatedActors))
  (CallFunction|FindBestPerceptedActorbySight _output_get))

(event EventOnPossess
  (params (PossessedPawn :type Pawn%20Object%20Reference))
  (|CallParentFunction PossessedPawn)
  ;[1 1 1] Run Behavior Tree
  (AI|RunBehaviorTree "/Game/Gameplay/Controller/AIController/AI_COBehaviorTree.AI_COBehaviorTree"))

(event EventBeginPlay)

(event EventTick
  (params (DeltaSeconds :type Float%20%28single-precision%29)))

(event EventOnTargetDeath
  ;[1 1 1] The new target is the current target or the last sound heard
  (CallFunction|FindBestPerceptedActorbySight (Variables|Default|GetPerceptedActors)))

(fn ConstructionScript)

(fn FindBestPerceptedActorbySight
  (params (PerceptedActors :type Array%20of%20Actor%20Object%20References))
  (Utilities|FlowControl|Sequence
    (:then_1
      (bind _targetactor (CallFunction|GetTargetActorBlackboard))
      (bind _output_get (LocalVariables|SetLocalTargetActor _targetactor))
      (Utilities|IsValid _output_get
        (:Is%20Valid
          (bind (_info _returnvalue) (Class|AIPerceptionComponent|GetActorsPerception (Variables|Default|GetAIPerception) (LocalVariables|GetLocalTargetActor)))
          (if _returnvalue ; Still sensed
            ;[1 1 1] Is sight stimulus valid?
            (if (< (.Age (Utilities|Struct|BreakAIStimulus (Utilities|Array|Get(acopy) (.LastSensedStimuli (Utilities|Struct|BreakActorPerceptionBlueprintInfo _info))))) (Variables|Default|GetDefaultSearchTime))
              (if (.bSuccessfullySensed (Utilities|Struct|BreakAIStimulus (Utilities|Array|Get(acopy) (.LastSensedStimuli (Utilities|Struct|BreakActorPerceptionBlueprintInfo _info)))))
                ;[1 1 1] If the actor is dead?
                (Utilities|IsActorDead? (LocalVariables|GetLocalTargetActor)
                  (:IsAlive
                    ;[1 1 1] Refind target
                    (CallFunction|SetActorFoundinBlackboard (LocalVariables|GetLocalTargetActor))
                    (return (LocalVariables|GetLocalTargetActor)))
                  (:IsDead
                    _))
                (else
                  ;[1 1 1] If the actor is dead?
                  (Utilities|IsActorDead? (LocalVariables|GetLocalTargetActor) :!label _label
                    (:IsAlive
                      ;[1 1 1] Target Lost
                      (CallFunction|SetActorLostinBlackboard (Variables|Default|GetDefaultSearchTime))
                      (return 0))
                    (:IsDead
                      _))))
              ;[1 1 1] Target is dead
              (CallFunction|SetActorLostinBlackboard 0.0))))))
    (:then_2
      (for _array_element PerceptedActors
        (bind _output_get_2 (LocalVariables|SetTempActor _array_element))
        (bind _info_2 (Class|AIPerceptionComponent|GetActorsPerception (Variables|Default|GetAIPerception) _output_get_2))
        (for (_array_element_2 _array_index) (.LastSensedStimuli (Utilities|Struct|BreakActorPerceptionBlueprintInfo _info_2))
          ;[1 1 1] If the sense is sight
          (if (== _array_index 0)
            (if (.bSuccessfullySensed (Utilities|Struct|BreakAIStimulus _array_element_2))
              ;[1 1 1] If the actor is dead?
              (Utilities|IsActorDead? (LocalVariables|GetTempActor)
                (:IsAlive
                  ;[1 1 1] Sucessfully find an actor
                  (CallFunction|SetActorFoundinBlackboard (LocalVariables|GetTempActor))
                  (return (LocalVariables|GetTempActor))))))))
      ;[1 1 1] If we find a better actor by sound
      (bind _bestactorbysound (CallFunction|FindBestPerceptedActorbySound PerceptedActors))
      (Utilities|IsValid _bestactorbysound
        (:Is%20Valid
          (CallFunction|SetActorFoundinBlackboard _bestactorbysound)
          (CallFunction|SetActorLostinBlackboard (Variables|Default|GetDefaultSearchTime))
          (return _bestactorbysound))
        (:Is%20Not%20Valid
          (goto _label))))))

(fn SetActorFoundinBlackboard
  (params (NewActorFound :type Object%20Object%20Reference))
  (bind _returnvalue (AI|GetBlackboard 0))
  (AI|Components|Blackboard|SetValueasObject _returnvalue (Variables|Default|GetTargetActorBlackboardKey) NewActorFound)
  (AI|Components|Blackboard|SetValueasBool _returnvalue (Variables|Default|GetTargetActorIsSightByAiPerceptionBlackBoardKey) true)
  (return))

(fn SetActorLostinBlackboard
  (params (SearchTime :type Float%20%28single-precision%29))
  (bind _returnvalue (AI|GetBlackboard 0))
  (bind _returnvalue_2 (AI|GetBlackboard 0))
  (if (<= SearchTime 0.0)
    (AI|Components|Blackboard|SetValueasBool _returnvalue_2 (Variables|Default|GetTargetActorIsSightByAiPerceptionBlackBoardKey) false)
    (AI|Components|Blackboard|SetValueasFloat _returnvalue_2 (Variables|Default|GetSearchTimeBlackboardKey) 0.0)
    (AI|Components|Blackboard|SetValueasObject _returnvalue_2 (Variables|Default|GetTargetActorBlackboardKey) 0)
    (return)
    (else
      (AI|Components|Blackboard|SetValueasBool _returnvalue (Variables|Default|GetTargetActorIsSightByAiPerceptionBlackBoardKey) false)
      (AI|Components|Blackboard|SetValueasFloat _returnvalue (Variables|Default|GetSearchTimeBlackboardKey) SearchTime)
      (return))))

(fn GetTargetActorBlackboard
  (bind _returnvalue (AI|GetBlackboard 0))
  (bind _targetactorblackboardkey (Variables|Default|GetTargetActorBlackboardKey))
  (bind _returnvalue_2 (AI|Components|Blackboard|GetValueasObject _returnvalue _targetactorblackboardkey))
  (Utilities|IsValid _returnvalue_2
    (:Is%20Valid
      (bind _asactor (Utilities|Casting|CastToActor _returnvalue_2)
        (:then
          (return _asactor))
        (:CastFailed
          _)))
    (:Is%20Not%20Valid
      _))
  (return 0))

(fn GetAcceptanceRadiusinCombat
  (return 1.5e+03))

(fn FindBestPerceptedActorbySound
  (params (PerceptedActors :type Array%20of%20Actor%20Object%20References))
  (for _array_element PerceptedActors
    (Utilities|IsActorDead? _array_element
      (:IsAlive
        (if (!= _array_element (Pawn|GetControlledPawn))
          (bind (_info _returnvalue) (Class|AIPerceptionComponent|GetActorsPerception (Variables|Default|GetAIPerception) _array_element))
          (if _returnvalue
            (Utilities|IsValid (LocalVariables|GetbestPerceptedActor)
              (:Is%20Valid
                (if (Math|Boolean|ANDBoolean (> (Variables|Default|GetDefaultSearchTime) (.Age (Utilities|Struct|BreakAIStimulus (Utilities|Array|Get(acopy) (.LastSensedStimuli (Utilities|Struct|BreakActorPerceptionBlueprintInfo _info)) 1)))) (.bSuccessfullySensed (Utilities|Struct|BreakAIStimulus (Utilities|Array|Get(acopy) (.LastSensedStimuli (Utilities|Struct|BreakActorPerceptionBlueprintInfo _info)) 1))) (> (LocalVariables|GetBestPerceptedActorDistance) (Math|Vector|VectorLength (- (.StimulusLocation (Utilities|Struct|BreakAIStimulus (Utilities|Array|Get(acopy) (.LastSensedStimuli (Utilities|Struct|BreakActorPerceptionBlueprintInfo _info)) 1))) (.ReceiverLocation (Utilities|Struct|BreakAIStimulus (Utilities|Array|Get(acopy) (.LastSensedStimuli (Utilities|Struct|BreakActorPerceptionBlueprintInfo _info)) 1)))))))
                  (LocalVariables|SetbestPerceptedActor _array_element :!label _label)
                  (LocalVariables|SetBestPerceptedActorDistance (Math|Vector|VectorLength (- (.StimulusLocation (Utilities|Struct|BreakAIStimulus (Utilities|Array|Get(acopy) (.LastSensedStimuli (Utilities|Struct|BreakActorPerceptionBlueprintInfo _info)) 1))) (.ReceiverLocation (Utilities|Struct|BreakAIStimulus (Utilities|Array|Get(acopy) (.LastSensedStimuli (Utilities|Struct|BreakActorPerceptionBlueprintInfo _info)) 1))))))))
              (:Is%20Not%20Valid
                ;[1 1 1] Init
                (if (and (> (Variables|Default|GetDefaultSearchTime) (.Age (Utilities|Struct|BreakAIStimulus (Utilities|Array|Get(acopy) (.LastSensedStimuli (Utilities|Struct|BreakActorPerceptionBlueprintInfo _info)) 1)))) (.bSuccessfullySensed (Utilities|Struct|BreakAIStimulus (Utilities|Array|Get(acopy) (.LastSensedStimuli (Utilities|Struct|BreakActorPerceptionBlueprintInfo _info)) 1))))
                  (goto _label)))))))))
  (return (LocalVariables|GetbestPerceptedActor)))