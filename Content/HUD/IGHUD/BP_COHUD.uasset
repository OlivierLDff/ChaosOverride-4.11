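; BP_COHUD is the in-game HUD for COCharacter pawns, drawing the aiming crosshair and hosting the main HUD widget.
; DrawHUD draws a centred crosshair texture while aiming, switching texture when the character has a target.
; A DoOnce creates the IGHUD widget and seeds its kill board with two rows using the owner's PlayerState.
; When the pawn is not a COCharacter, DrawHUD removes the widget and resets the DoOnce.
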(event `self.ReceiveBeginPlay`
  (`KismetSystemLibrary.Delay` 3.0)
  (bind _ascocharacter (cast `COCharacter` (`self.GetOwningPawn`))
    (:`then`
      (set `self.COCharacterOwner` _ascocharacter))
    (:`CastFailed`
      (`KismetSystemLibrary.PrintString` "Error : You are using this HUD with the wrong pawn type")
      (`self.K2_DestroyActor` self))))

(event `self.ReceiveActorBeginOverlap`
  (params (OtherActor :type "Actor Object Reference")))

(event `self.ReceiveTick`
  (params (DeltaSeconds :type "Float (single-precision)")))

(event `self.ReceiveDrawHUD`
  (params (SizeX :type Integer) (SizeY :type Integer))
  (bind _returnvalue (`self.GetOwningPlayerController`))
  (bind _cocharacterowner (`self.COCharacterOwner`))
  (bind _hudwidget (`self.HUDWidget`))
  (bind _returnvalue_2 (`KismetMathLibrary.Conv_IntToDouble` (- (/ SizeX 2) 16)))
  (bind _returnvalue_3 (`KismetMathLibrary.Conv_IntToDouble` (- (/ SizeY 2) 16)))
  (bind _ascocharacter (cast `COCharacter` (`self.GetOwningPawn`))
    (:`then`
      (set `self.COCharacterOwner` _ascocharacter)
      (`|ExecutionSequence`
        (:`then_0`
          (if (`COCharacter.bIsAiming` _cocharacterowner)
            (if (`COCharacter.HasATarget` _cocharacterowner)
              (`self.DrawTextureSimple` "/Game/HUD/IGHUD/T_Cross2.T_Cross2" _returnvalue_2 _returnvalue_3 1.0)
              (else
                (`self.DrawTextureSimple` "/Game/HUD/IGHUD/T_Cross1.T_Cross1" _returnvalue_2 _returnvalue_3 1.0)))))
        (:`then_1`
          (`/Engine/EditorBlueprintResources/StandardMacros.DoOnce` false :!label _label
            (:`Completed`
              (bind _returnvalue_4 (`Controller.CastToPlayerController` (`Pawn.GetController` _cocharacterowner)))
              (bind _returnvalue_5 (`|CreateWidget` "/Game/HUD/IGHUD/IGHUDWIdget.IGHUDWIdget_C" _returnvalue_4 _cocharacterowner))
              (bind _output_get (set `self.HUDWidget` _returnvalue_5))
              (`UserWidget.AddToPlayerScreen` _output_get 0)
              (bind _asbp_coplayer_state (cast `/Game/Gameplay/Controller/BP_COPlayerState` (`Pawn.PlayerState` (`self.COCharacterOwner`))))
              (bind _returnvalue_6 (`|CreateWidget` "/Game/HUD/IGHUD/Killboard/W_KillBoardRow.W_KillBoardRow_C" _returnvalue _asbp_coplayer_state _asbp_coplayer_state))
              (`PanelWidget.AddChild` (`/Game/HUD/IGHUD/Killboard/W_KillBoard.KillboardBox` (`/Game/HUD/IGHUD/IGHUDWIdget.W_KillBoard` (`self.HUDWidget`))) _returnvalue_6)
              (bind _returnvalue_7 (`|CreateWidget` "/Game/HUD/IGHUD/Killboard/W_KillBoardRow.W_KillBoardRow_C" _returnvalue _asbp_coplayer_state))
              (`PanelWidget.AddChild` (`/Game/HUD/IGHUD/Killboard/W_KillBoard.KillboardBox` (`/Game/HUD/IGHUD/IGHUDWIdget.W_KillBoard` (`self.HUDWidget`))) _returnvalue_7))))))
    (:`CastFailed`
      (`/Engine/EditorBlueprintResources/StandardMacros.IsValid` _hudwidget
        (:`Is Valid`
          (`Widget.RemoveFromParent` _hudwidget)
          (goto _label :!via `Reset`))))))

(fn `UserConstructionScript`)