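; Projectile actor for the Devastator weapon that deals point damage to pawns and then destroys itself.
; Each Tick it runs a short complex sphere trace for Pawn objects just ahead of its root, and a hit triggers the damage.
; The damaged actor is taken from the ActorBeginOverlap pin rather than the trace result, though that event itself does nothing.
; An older channel trace and a plain ApplyDamage remain disconnected.
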(event `self.ReceiveBeginPlay`)

(event `self.ReceiveActorBeginOverlap`
  (params (OtherActor :type "Actor Object Reference"))
  (if true
    (if true
      _)))

(event `self.ReceiveTick`
  (params (DeltaSeconds :type "Float (single-precision)"))
  (bind _returnvalue (`self.GetActorForwardVector`))
  (bind _returnvalue_2 (`SceneComponent.K2_GetComponentLocation` (`self.Root`)))
  (bind (_outhit _returnvalue_3) (`KismetSystemLibrary.SphereTraceSingleForObjects` _returnvalue_2 (+ _returnvalue_2 (* _returnvalue 1.0)) 20.0 (`|MakeArray` "ObjectTypeQuery3" :!type "EObjectTypeQuery Enum") true))
  (if _returnvalue_3
    (`GameplayStatics.ApplyPointDamage` (stale `self.ReceiveActorBeginOverlap` OtherActor) 20.0 _returnvalue _outhit (`self.GetInstigatorController`) (`self.GetInstigator`) "/Script/Engine.DamageType")
    (`self.K2_DestroyActor`)))

(fn `UserConstructionScript`)