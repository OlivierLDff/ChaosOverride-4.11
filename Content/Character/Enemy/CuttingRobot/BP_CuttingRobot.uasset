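; BP_CuttingRobot is an enemy that chases the player and damages other actors that begin overlapping its sphere.
; A custom event loops AI MoveTo toward the player pawn, restarting on success or failure.
; The first damage of any amount triggers an explosion and teleports it below the level.
; After a short delay, it spawns a replacement at a random TargetPoint and destroys itself, only if any TargetPoint exists.
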(event `CustomEvent_0`
  (`|AIMoveTo` self (0.0 0.0 0.0) (`GameplayStatics.GetPlayerPawn` 0)
    (:`OnSuccess`
      _)
    (:`OnFail`
      _))
  (`self.CustomEvent_0`))

(event `self.ReceiveBeginPlay`
  (`self.CustomEvent_0`))

(event `self.ReceiveActorBeginOverlap`
  (params (OtherActor :type "Actor Object Reference")))

(event `self.ReceiveTick`
  (params (DeltaSeconds :type "Float (single-precision)")))

(event `self.Sphere.OnComponentBeginOverlap`
  (params (OtherActor :type "Actor Object Reference") (OtherComp :type "PrimitiveComponent Object Reference") (OtherBodyIndex :type Integer) (bFromSweep :type Boolean) (SweepResult :type "HitResult Structure (by ref)"))
  (if (not (== OtherActor self))
    (`GameplayStatics.ApplyDamage` OtherActor 10.0 (`self.GetController`) self "/Script/ChaosOverride.CODamageType")))

(event `self.ReceiveAnyDamage`
  (params (Damage :type "Float (single-precision)") (DamageType :type "DamageType Object Reference") (InstigatedBy :type "Controller Object Reference") (DamageCauser :type "Actor Object Reference"))
  (bind _returnvalue (`self.K2_GetActorLocation`))
  (`/Engine/EditorBlueprintResources/StandardMacros.DoOnce` false
    (:`Completed`
      (`GameplayStatics.SpawnSoundAtLocation` "/Game/StarterContent/Audio/Explosion01.Explosion01" _returnvalue)
      (`GameplayStatics.SpawnEmitterAtLocation` "/Game/StarterContent/Particles/P_Explosion.P_Explosion" _returnvalue)
      (`self.K2_SetActorLocation` (0.0 0.0 -500.0) false true)
      (`KismetSystemLibrary.Delay` 1.0)
      (bind _outactors (`GameplayStatics.GetAllActorsOfClass` "/Script/Engine.TargetPoint"))
      (bind _returnvalue_2 (`KismetArrayLibrary.Array_Length` _outactors))
      (if (!= _returnvalue_2 0)
        (`|SpawnActorFromClass` "BP_CuttingRobot_C" (`self.GetTransform` (`KismetArrayLibrary.Array_Get` _outactors (`KismetMathLibrary.RandomIntegerInRange` 0 (- _returnvalue_2 1)))) "AlwaysSpawn" "OverrideRootScale")
        (`self.K2_DestroyActor`)))))

(fn `UserConstructionScript`)